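; L_WindowBP is an interactive window actor that slides down and up while control buttons are held.
; On BeginPlay it passes itself to its L_WindowControl widget and records the window's starting relative location.
; Button presses play or reverse the WindowAnimation timeline, and releases stop it, leaving the window partway.
; The timeline lerps LWindow between that start and a point 220 units lower in Z.
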(event Custom|Up%20Button%20Released
  (bind _window_start_position (Variables|Default|GetWindow%20Start%20Position))
  (bind _newtrack_0 (Timeline|Window%20Animation Stop)
    (:Update
      (Transformation|SetRelativeLocation (Variables|Default|GetL_Window) (Math|Vector|Lerp(Vector) _window_start_position (+ _window_start_position "0,0.000000,-220.000000") _newtrack_0) false false))))

(event Custom|Up%20Button%20Pressed
  (bind _window_start_position (Variables|Default|GetWindow%20Start%20Position))
  (bind _newtrack_0 (Timeline|Window%20Animation Reverse)
    (:Update
      (Transformation|SetRelativeLocation (Variables|Default|GetL_Window) (Math|Vector|Lerp(Vector) _window_start_position (+ _window_start_position "0,0.000000,-220.000000") _newtrack_0) false false))))

(event Custom|Down%20Button%20Pressed
  (bind _window_start_position (Variables|Default|GetWindow%20Start%20Position))
  (bind _newtrack_0 (Timeline|Window%20Animation Play)
    (:Update
      (Transformation|SetRelativeLocation (Variables|Default|GetL_Window) (Math|Vector|Lerp(Vector) _window_start_position (+ _window_start_position "0,0.000000,-220.000000") _newtrack_0) false false))))

(event Custom|Down%20Button%20Released
  (bind _window_start_position (Variables|Default|GetWindow%20Start%20Position))
  (bind _newtrack_0 (Timeline|Window%20Animation Stop)
    (:Update
      (Transformation|SetRelativeLocation (Variables|Default|GetL_Window) (Math|Vector|Lerp(Vector) _window_start_position (+ _window_start_position "0,0.000000,-220.000000") _newtrack_0) false false))))

(event EventBeginPlay
  (|CallParentFunction)
  (bind _asl_window_control (Utilities|Casting|CastToL_WindowControl (UserInterface|GetUserWidgetObject (Variables|Default|GetWidget))))
  (Default|SetParent _asl_window_control self)
  (Variables|Default|SetWindow%20Start%20Position (Variables|/Script/Engine.SceneComponent|GetRelativeLocation (Variables|Default|GetL_Window))))

(fn ConstructionScript
  (|CallParentFunction))